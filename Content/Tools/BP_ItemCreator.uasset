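; BP_ItemCreator is a tool Blueprint that generates and saves item pickup assets from item data and item logic.
; GenerateItemPickup creates the pickup, runs the target path through FilePathProcessor, saves it under the given file name and logs a debug "Hello".
; The EventGraph and CreatePickupMacro hold copies of the same create-and-save chain that never run.
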(fn `GenerateItemPickup`
  (params (ItemData :type "DA_ZAQItemData Class Reference") (ItemLogic :type "ZAQItem Class Reference") (FilePath :type "FilePath Structure") (FileName :type String))
  (bind _returnvalue (`self.CreatePickupItem` ItemData ItemLogic))
  (bind _returnvalue_2 (`self.FilePathProcessor` FilePath))
  (`self.SaveItemPickup` _returnvalue _returnvalue_2 FileName)
  (`KismetSystemLibrary.LogString` "Hello"))